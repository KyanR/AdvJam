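; Interactive door handle that turns and springs back when its Open event is called.
; BeginPlay stores the actor's starting rotation and derives a turned rotation from per-axis offsets.
; Open chains two timelines that lerp the actor to the turned rotation and back along sigmoid-named curves.
; It flags movement during the animation and marks the handle as opened when the return finishes.
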(event `self.ReceiveBeginPlay`
  ;[1 0.1779 0.1779] Setting up the initial and final position
  (bind _output_get (set `self.Initial_Handle_Rotation` (`self.K2_GetActorRotation`)))
  (set `self.Final_Handle_Rotation` (`KismetMathLibrary.MakeRotator` (+ (.roll _output_get) (`self.X_Offset_Handle_World_Rotation`)) (+ (.pitch _output_get) (`self.Y_Offset_Handle_World_Rotation`)) (+ (.yaw _output_get) (`self.Z_Offset_Handle_World_Rotation`)))))

(event `Open`
  ;[1 0.5333 0.007843] Open event for door
  (set `self.Is_In_Movement` true)
  (bind (_direction _sigm_function) (`Timeline|Open_TimeLine` :!via `PlayFromStart`)
    (:`Update`
      (`self.K2_SetActorRotation` (`KismetMathLibrary.RLerp` (`self.Initial_Handle_Rotation`) (`self.Final_Handle_Rotation`) _sigm_function true)))
    (:`Finished`
      (bind (_direction_2 _sigm_funct) (`Timeline|Open_TimeLine_2` :!via `PlayFromStart`)
        (:`Update`
          (`self.K2_SetActorRotation` (`KismetMathLibrary.RLerp` (`self.Final_Handle_Rotation`) (`self.Initial_Handle_Rotation`) _sigm_funct true)))
        (:`Finished`
          (set `self.Is_Already_Opened` true)
          (set `self.Is_In_Movement` false))))))

(fn `UserConstructionScript`
  (`parent.UserConstructionScript`))