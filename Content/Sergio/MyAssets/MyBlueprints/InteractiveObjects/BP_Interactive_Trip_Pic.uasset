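; BP_Interactive_Trip_Pic is an interactive mountain trip picture that plays a memory as on-screen dialogue.
; Play_Memory sets IsPlayed, adds a Dialogue_Interface widget to the viewport and disables player input, with no re-enable here.
; It loops the widget's MountainTripDialoguesArray into the dialogue text, but the Delay inside the loop does not pace lines, so the last entry shows immediately.
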(event `Play_Memory`
  (bind _dialogue_interface (`self.Dialogue_Interface`))
  ;[0.9107 0.3733 1] - Trip mountain picture interaction -
  (set `self.Is_Played` true)
  (bind _returnvalue (`|CreateWidget` "/Game/Sergio/MyAssets/MyBlueprints/DialogueSystem/Dialogue_Interface.Dialogue_Interface_C"))
  (bind _output_get (set `self.Dialogue_Interface` _returnvalue))
  (`UserWidget.AddToViewport` _output_get 0)
  (`self.DisableInput` (`GameplayStatics.GetPlayerCharacter` 0) (`GameplayStatics.GetPlayerController` 0))
  (for _array_element (`/Game/Sergio/MyAssets/MyBlueprints/DialogueSystem/Dialogue_Interface.Mountain_Trip_Dialogues_Array` _dialogue_interface)
    (`TextBlock.SetText` (`/Game/Sergio/MyAssets/MyBlueprints/DialogueSystem/Dialogue_Interface.Main_Dialogue_Conver` _dialogue_interface) _array_element)
    (`KismetSystemLibrary.Delay` 1.0)
    (`KismetSystemLibrary.PrintString` (`KismetTextLibrary.Conv_TextToString` _array_element))))

(event `Test`)

(fn `UserConstructionScript`
  (`parent.UserConstructionScript`))