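; Interactive door actor that swings open by rotating the whole actor from its starting rotation to an offset one.
; BeginPlay stores the initial rotation and builds the final one by adding per-axis offset variables.
; The Open event plays a timeline whose SigmFunction track drives a shortest-path rotator lerp, flagging the door as moving, then as opened when finished.
; No close logic is present.
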(event `self.ReceiveBeginPlay`
  ;[1 0.1779 0.1779] Setting up the initial and final handle and door position/rotation
  (bind _output_get (set `self.Initial_Door_Position` (`self.K2_GetActorRotation`)))
  (set `self.Final_Door_Position` (`KismetMathLibrary.MakeRotator` (+ (.roll _output_get) (`self.X_Offset_Door_World_Rotation`)) (+ (.pitch _output_get) (`self.Y_Offset_Door_World_Rotation`)) (+ (.yaw _output_get) (`self.Z_Offset_Door_World_Rotation_0`)))))

(event `Open`
  ;[1 0.5333 0.007843] Open event for door
  (set `self.Is_In_Movement` true)
  (bind (_direction _sigm_function) (`Timeline|Timeline_0` :!via `PlayFromStart`)
    (:`Update`
      (`self.K2_SetActorRotation` (`KismetMathLibrary.RLerp` (`self.Initial_Door_Position`) (`self.Final_Door_Position`) _sigm_function true))
      (`/Engine/EditorBlueprintResources/StandardMacros.DoOnce` false))
    (:`Finished`
      (set `self.Is_In_Movement` false)
      (set `self.Is_Already_Opened` true))))

(fn `UserConstructionScript`
  (`parent.UserConstructionScript`))