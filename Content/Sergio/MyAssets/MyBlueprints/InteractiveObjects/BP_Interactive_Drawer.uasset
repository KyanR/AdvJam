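; Interactive drawer actor that slides open and closed with matching sounds.
; BeginPlay stores the start location and adds configurable XYZ offsets to get the open position.
; Open and Close events each run a timeline that lerps the actor between both positions and updates InMovement and AlreadyOpened state.
; Cross-resetting DoOnce nodes make each sound play once per movement as the drawer alternates between opening and closing.
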(event `self.ReceiveBeginPlay`
  ;[1 0.1779 0.1779] Setting up the initial and final position
  (bind _output_get (set `self.Initial_Position` (`self.K2_GetActorLocation`)))
  (set `self.Final_Position` (+ _output_get (`KismetMathLibrary.MakeVector` (`self.X_Offset_World_Position`) (`self.Y_Offset_World_Position`) (`self.Z_Offset_World_Position`)))))

(event `Open`
  ;[1 0.5333 0.007843] Open event for drawer
  (set `self.In_Movement` true)
  (bind (_direction _sigm_function) (`Timeline|Open_TimeLine` :!via `PlayFromStart`)
    (:`Update`
      (`self.K2_SetActorRelativeLocation` (`KismetMathLibrary.VLerp` (`self.Initial_Position`) (`self.Final_Position`) _sigm_function))
      (`/Engine/EditorBlueprintResources/StandardMacros.DoOnce` false :!label _label
        (:`Completed`
          (`AudioComponent.Play` (`self.DrawOpen`) 0.0)
          (goto _label_2 :!via `Reset`))))
    (:`Finished`
      (set `self.Already_Opened` true)
      (set `self.In_Movement` false))))

(event `Close`
  ;[1 0.5333 0.007843] Close event for drawer
  (set `self.In_Movement` true)
  (bind (_direction _sigm_function) (`Timeline|Timeline_0` :!via `PlayFromStart`)
    (:`Update`
      (`self.K2_SetActorRelativeLocation` (`KismetMathLibrary.VLerp` (`self.Final_Position`) (`self.Initial_Position`) _sigm_function))
      (`/Engine/EditorBlueprintResources/StandardMacros.DoOnce` false :!label _label_2
        (:`Completed`
          (`AudioComponent.Play` (`self.DrawClose`) 0.0)
          (goto _label :!via `Reset`))))
    (:`Finished`
      (set `self.Already_Opened` false)
      (set `self.In_Movement` false))))

(fn `UserConstructionScript`
  (`parent.UserConstructionScript`))