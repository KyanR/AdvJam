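; BP_Interact_Master is an interactable actor, apparently a base class by its name, that announces itself to actors entering its Trigger.
; Trigger begin overlap sends SetInteracObjectMessage to the other actor with itself as the argument, and end overlap sends it empty to clear the reference.
; GetAction exposes the Action variable.
; Unconnected leftover nodes cast to BP_Veronica for spot detected and release notifications and never run.
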(event `self.Trigger.OnComponentBeginOverlap`
  (params (OverlappedComponent :type "PrimitiveComponent Object Reference") (OtherActor :type "Actor Object Reference") (OtherComp :type "PrimitiveComponent Object Reference") (OtherBodyIndex :type Integer) (bFromSweep :type Boolean) (SweepResult :type "HitResult Structure (by ref)"))
  (message `/Game/TJ/Blueprint/Interface/BPI_Veronica.SetInteracObject` OtherActor self))

(event `self.Trigger.OnComponentEndOverlap`
  (params (OverlappedComponent :type "PrimitiveComponent Object Reference") (OtherActor :type "Actor Object Reference") (OtherComp :type "PrimitiveComponent Object Reference") (OtherBodyIndex :type Integer))
  (message `/Game/TJ/Blueprint/Interface/BPI_Veronica.SetInteracObject` OtherActor null))

(fn `GetAction`
  (returns (PickUpFrame :type String))
  (return (`self.Action`)))

(fn `UserConstructionScript`)