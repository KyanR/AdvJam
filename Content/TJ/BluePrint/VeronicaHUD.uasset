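; VeronicaHUD is a HUD Blueprint that shows and hides item interaction messages on screen.
; On BeginPlay it creates a VeronicaInterface widget for the first player controller, stores the reference and adds it to the viewport.
; Its notify events forward display and hide requests to that widget, with BuildInteractionMessage forming the text by prefixing "E" to the lowercased item name.
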(event `self.ReceiveBeginPlay`
  ;[1 1 1] Add UI Messages on ViewPort
  (bind _returnvalue (`|CreateWidget` "/Game/TJ/Blueprint/VeronicaInterface.VeronicaInterface_C" (`GameplayStatics.GetPlayerController` 0)))
  (bind _output_get (set `self.UIMessagesRef` _returnvalue))
  (`UserWidget.AddToViewport` _output_get 0))

(event `Notify Display Interact Message`
  (params (Item :type Name))
  ;[1 1 1] Notofication
  (bind _message (`self.BuildInteractionMessage` Item))
  (`/Game/TJ/Blueprint/VeronicaInterface.DisplayInteractionMessage` (`self.UIMessagesRef`) _message))

(event `Notify Hide Interaction Message`
  ;[1 1 1] Notofication
  (`/Game/TJ/Blueprint/VeronicaInterface.HiddenInteractionMessage` (`self.UIMessagesRef`)))

(event `self.ReceiveDrawHUD`
  (params (SizeX :type Integer) (SizeY :type Integer)))

(fn `BuildInteractionMessage`
  (params (`Name of Item` :type Name))
  (returns (Message :type Text))
  (return (`KismetTextLibrary.Conv_StringToText` (`KismetStringLibrary.Concat_StrStr` "E" (`KismetStringLibrary.ToLower` (`KismetStringLibrary.Conv_NameToString` `Name of Item`))))))

(fn `UserConstructionScript`)